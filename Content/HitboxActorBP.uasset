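; Hitbox actor for a two-player fighting game that displays a proximity, strike or hurtbox volume and applies damage to the opponent.
; SpawnHitbox sets a material by HitboxType, moves the display to HitboxLocation, makes it visible, then runs CheckCollision once.
; CheckCollision compares its owner to Player1 in DefaultGameMode to pick the opponent, then applies HitboxDamage if overlapping that player's Hurtbox, regardless of hitbox type.
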(event `SpawnHitbox`
  (bind _hitboxdisplay (`self.HitboxDisplay`))
  (switch `EHitboxEnum` (`self.hitboxType`)
    (:`HB_PROXIMITY`
      (`PrimitiveComponent.SetMaterial` _hitboxdisplay 0 "/Game/M_ProximityHitbox.M_ProximityHitbox"))
    (:`HB_STRIKE`
      (`PrimitiveComponent.SetMaterial` _hitboxdisplay 0 "/Game/M_ActiveHitbox.M_ActiveHitbox"))
    (:`HB_HURTBOX`
      (`PrimitiveComponent.SetMaterial` _hitboxdisplay 0 "/Game/M_Hurtbox.M_Hurtbox")))
  (`SceneComponent.K2_SetWorldLocation` (`self.HitboxDisplay`) (`self.hitboxLocation`) false false)
  (`SceneComponent.SetVisibility` (`self.HitboxDisplay`) true false)
  (`self.CheckCollision`))

(event `CheckCollision`
  (bind _player2 (`BAFG_CaliburstGameMode.player2` (`self.GameModeRef`)))
  (bind _player1 (`BAFG_CaliburstGameMode.player1` (`self.GameModeRef`)))
  (bind _asdefault_game_mode (cast `/Game/Blueprint/DefaultGameMode` (`GameplayStatics.GetGameMode`)))
  (set `self.GameModeRef` _asdefault_game_mode)
  (bind _isp1 (`self.DeterminePlayer`))
  (if _isp1
    (if (`self.IsOverlappingActor` (`BAFG_CaliburstCharacter.hurtbox` _player2))
      (`BAFG_CaliburstCharacter.TakeDamage` _player2 (`self.hitboxDamage`)))
    (elif (`self.IsOverlappingActor` (`BAFG_CaliburstCharacter.hurtbox` _player1))
      (`BAFG_CaliburstCharacter.TakeDamage` _player1 (`self.hitboxDamage`)))))

(fn `DeterminePlayer`
  (returns (IsP1 :type Boolean))
  (return (== (`BAFG_CaliburstGameMode.player1` (`self.GameModeRef`)) (`self.GetOwner`))))

(fn `UserConstructionScript`)