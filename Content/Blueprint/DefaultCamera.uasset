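; Shared camera actor that keeps two players in frame along the Y-Z plane.
; After a short delay on BeginPlay, it caches both player references from DefaultGameMode.
; Each tick it holds its X, centers on the players' Y midpoint and sets Z from their summed heights, using a divisor below two.
; ZoomControl then scales field of view with their horizontal separation, clamped to a fixed range.
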(event `self.ReceiveBeginPlay`
  (`KismetSystemLibrary.Delay` 0.1)
  (bind _asdefault_game_mode (cast `/Game/Blueprint/DefaultGameMode` (`GameplayStatics.GetGameMode`)))
  (bind _output_get (set `self.GameModeRef` _asdefault_game_mode))
  (bind _player1 (`BAFG_CaliburstGameMode.player1` _output_get))
  (bind _player2 (`BAFG_CaliburstGameMode.player2` _output_get))
  (if (and (`KismetSystemLibrary.IsValid` _player1) (`KismetSystemLibrary.IsValid` _player2))
    (set `self.P1Ref` _player1)
    (set `self.P2Ref` _player2)))

(event `self.ReceiveTick`
  (params (DeltaSeconds :type "Float (single-precision)"))
  (bind _returnvalue_x (`KismetMathLibrary.BreakVector` (`self.K2_GetActorLocation`)))
  (bind _p1ref (`self.P1Ref`))
  (bind _p2ref (`self.P2Ref`))
  (if (and (`KismetSystemLibrary.IsValid` _p1ref) (`KismetSystemLibrary.IsValid` _p2ref))
    (`self.K2_SetActorLocation` (`KismetMathLibrary.MakeVector` _returnvalue_x (/ (+ (.y (`self.K2_GetActorLocation` _p1ref)) (.y (`self.K2_GetActorLocation` _p2ref))) 2.0) (/ (+ (.z (`self.K2_GetActorLocation` _p1ref)) (.z (`self.K2_GetActorLocation` _p2ref))) 1.7)))
    (`self.ZoomControl`)))

(fn `UserConstructionScript`)

(fn `ZoomControl`
  (`CameraComponent.SetFieldOfView` (`self.CameraComponent`) (`KismetMathLibrary.FClamp` (`KismetMathLibrary.Abs` (* (- (.y (`self.K2_GetActorLocation` (`self.P1Ref`))) (.y (`self.K2_GetActorLocation` (`self.P2Ref`)))) 0.1)) 60.0 85.0)))