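; MenuGameMode is a game mode Blueprint whose BeginPlay is empty, leaving its match setup logic disconnected.
; The unused chain passes each PlayerStart to SpawnPlayers and adds a CharacterHUD widget.
; SpawnPlayers uses P1 and P2 tags to spawn characters through DetermineCharacterClass, which switches between SideScrollerCharacter and TestCharBP.
; Only Player1 gets possessed in that function, as the Player2 possession node is also disconnected.
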(event `self.ReceiveBeginPlay`)

(fn `DetermineCharacterClass`
  (params (Transform :type "Transform Structure") (Actor :type "Actor Object Reference"))
  (returns (ReturnValue :type "BAFG_CaliburstCharacter Object Reference"))
  (switch `ECharacterClass` "VE_Default"
    (:`VE_Default`
      (bind _returnvalue (`|SpawnActorFromClass` "/Game/SideScrollerCPP/Blueprints/SideScrollerCharacter.SideScrollerCharacter_C" Transform "Undefined" "OverrideRootScale" Actor null))
      (return _returnvalue))
    (:`VE_Char`
      (bind _returnvalue_2 (`|SpawnActorFromClass` "/Game/SideScrollerCPP/Blueprints/TestCharBP.TestCharBP_C" Transform "Undefined" "OverrideRootScale" Actor null))
      (return _returnvalue_2))))

(fn `SpawnPlayers`
  (params (Object :type "Actor Object Reference"))
  (bind _asplayer_start (cast `PlayerStart` Object))
  (if (== "P1" (`PlayerStart.PlayerStartTag` _asplayer_start))
    (bind _returnvalue (`self.DetermineCharacterClass` (`self.GetTransform` _asplayer_start) _asplayer_start))
    (bind _output_get (set `self.player1` _returnvalue))
    (`Controller.Possess` (`GameplayStatics.GetPlayerController` 0) _output_get)
    (elif (== "P2" (`PlayerStart.PlayerStartTag` _asplayer_start))
      (bind _returnvalue_2 (`self.DetermineCharacterClass` (`self.GetTransform` _asplayer_start) _asplayer_start))
      (bind _output_get_2 (set `self.player2` _returnvalue_2)))))

(fn `UserConstructionScript`)