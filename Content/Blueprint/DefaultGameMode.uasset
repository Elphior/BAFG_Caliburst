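; Game mode that spawns the two side-scroller player characters and shows the HUD when play begins.
; BeginPlay passes every PlayerStart to SpawnPlayers, which spawns a SideScrollerCharacter at those tagged P1 or P2 and stores it as Player1 or Player2.
; It then creates one CharacterHUD widget for player controller 0 and adds it to the viewport.
; The spawned characters are not explicitly possessed here.
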(event `self.ReceiveBeginPlay`
  (bind _outactors (`GameplayStatics.GetAllActorsOfClass` "/Script/Engine.PlayerStart"))
  (for _array_element _outactors
    (`self.SpawnPlayers` _array_element))
  (bind _returnvalue (`|CreateWidget` "/Game/Blueprint/UI/CharacterHUD.CharacterHUD_C" (`GameplayStatics.GetPlayerController` 0)))
  (`UserWidget.AddToViewport` _returnvalue 0))

(fn `SpawnPlayers`
  (params (Object :type "Actor Object Reference"))
  (bind _asplayer_start (cast `PlayerStart` Object))
  (if (== "P1" (`PlayerStart.PlayerStartTag` _asplayer_start))
    (bind _returnvalue (`|SpawnActorFromClass` "/Game/SideScrollerCPP/Blueprints/SideScrollerCharacter.SideScrollerCharacter_C" (`self.GetTransform` _asplayer_start) "Undefined" "OverrideRootScale" _asplayer_start null))
    (set `self.player1` _returnvalue)
    (elif (== "P2" (`PlayerStart.PlayerStartTag` _asplayer_start))
      (bind _returnvalue_2 (`|SpawnActorFromClass` "/Game/SideScrollerCPP/Blueprints/SideScrollerCharacter.SideScrollerCharacter_C" (`self.GetTransform` _asplayer_start) "Undefined" "OverrideRootScale" _asplayer_start null))
      (set `self.player2` _returnvalue_2))))

(fn `UserConstructionScript`)